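; Doodler player character that aims from the camera and paints on static meshes tagged Paintable.
; Tick traces forward from the camera, caching the hit and drawing a color-coded debug preview.
; Enhanced Input drives a timeline zoom of boom length and FOV, and feeds that hit to WallPaintingBrush, deactivating it on invalid targets or release.
; A helper, uncalled here, remaps hits to normalized mesh-local 2D coordinates.
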(event `self.ReceiveBeginPlay`
  (`parent.ReceiveBeginPlay`)
  (`EnhancedInputSubsystemInterface.AddMappingContext` (pcsubsystem `EnhancedInputLocalPlayerSubsystem` (`GameplayStatics.GetPlayerController` 0)) "/Game/Doodler/Blueprints/Input/IMC_DoodlerActions.IMC_DoodlerActions" 0 (struct)))

(event `EnhancedInput|/Game/Doodler/Blueprints/Input/IA_Zoom`
  (params (ActionValue :type Boolean) (ElapsedSeconds :type "Float (double-precision)") (TriggeredSeconds :type "Float (double-precision)") (InputAction :type "InputAction Object Reference" :default "/Game/Doodler/Blueprints/Input/IA_Zoom.IA_Zoom"))
  (:`Triggered`
    ;[1 1 1] camera zoom animation
    (`TimelineComponent.SetPlayRate` (`self.CameraZoomAnim`) (/ 1.0 1.5))
    (bind (_direction _alpha) (`Timeline|CameraZoomAnim` :!label _label)
      (:`Update`
        (set `SpringArmComponent.TargetArmLength` (`KismetMathLibrary.Lerp` 400.0 200.0 _alpha) (`self.CameraBoom`))
        (`CameraComponent.SetFieldOfView` (`self.FollowCamera`) (`KismetMathLibrary.Lerp` 90.0 70.0 _alpha)))))
  (:`Completed`
    (goto _label :!via `Reverse`)))

(event `EnhancedInput|/Game/Doodler/Blueprints/Input/IA_ShootPaint`
  (params (ActionValue :type Boolean) (ElapsedSeconds :type "Float (double-precision)") (TriggeredSeconds :type "Float (double-precision)") (InputAction :type "InputAction Object Reference" :default "/Game/Doodler/Blueprints/Input/IA_ShootPaint.IA_ShootPaint"))
  (bind _wallpaintingbrush (`self.WallPaintingBrush`))
  (bind (_bblockinghit _binitialoverlap _time _distance _location _impactpoint _normal _impactnormal _physmat _hitactor _hitcomponent) (`GameplayStatics.BreakHitResult` (`self.Out Hit`)))
  (:`Triggered`
    (if _bblockinghit
      (if (`ActorComponent.ComponentHasTag` _hitcomponent "Paintable")
        (bind _asstatic_mesh_component (cast `StaticMeshComponent` _hitcomponent)
          (:`then`
            (`MeshPaintingComponent.PreparePaintingData` _wallpaintingbrush _asstatic_mesh_component _location)
            (`ActorComponent.Activate` (`self.WallPaintingBrush`) false))
          (:`CastFailed`
            (`ActorComponent.Deactivate` _wallpaintingbrush :!label _label_2)))
        (else
          (goto _label_2)))
      (else
        (goto _label_2))))
  (:`Completed`
    (`ActorComponent.Deactivate` (`self.WallPaintingBrush`))))

(event `self.ReceiveTick`
  (params (DeltaSeconds :type "Float (single-precision)"))
  (bind _returnvalue (`GameplayStatics.GetPlayerCameraManager` 0))
  (bind _returnvalue_2 (`self.K2_GetActorLocation` _returnvalue))
  (`parent.ReceiveTick` DeltaSeconds)
  (bind _outhit (`KismetSystemLibrary.LineTraceSingle` :`Start` _returnvalue_2 :`End` (+ _returnvalue_2 (* 5000 (`self.GetActorForwardVector` _returnvalue))) :`TraceChannel` "TraceTypeQuery1" :`DrawTime` 0.15))
  (set `self.Out Hit` _outhit)
  (bind (_bblockinghit _binitialoverlap _time _distance _location _impactpoint _normal _impactnormal _physmat _hitactor _hitcomponent) (`GameplayStatics.BreakHitResult` _outhit))
  ;[1 1 1] preview only
  (`/Engine/EditorBlueprintResources/StandardMacros.IsValid` _hitcomponent
    (:`Is Valid`
      (`KismetSystemLibrary.DrawDebugSphere` _location 2.0 12 (`KismetMathLibrary.SelectColor` (struct :`G` 0.317708 :`B` 0.012663 :`A` 1.0) (struct :`R` 0.614583 :`A` 1.0) (`ActorComponent.ComponentHasTag` _hitcomponent "Paintable")) 0.0 5.0))))

(fn `RemapHitResultToLocalPainting`
  (params (Hit :type "HitResult Structure (by ref)"))
  (returns (NormalizedLocation :type "Vector2D Structure") (bIsValid :type Boolean))
  (bind (_bblockinghit _binitialoverlap _time _distance _location _impactpoint _normal _impactnormal _physmat _hitactor _hitcomponent) (`GameplayStatics.BreakHitResult` Hit))
  (bind (_extent_x _extent_y) (`KismetMathLibrary.BreakVector` (`self.Extent`)))
  (bind (_returnvalue_x _returnvalue_y) (`KismetMathLibrary.BreakVector` (- (0.0 0.0 0.0) (`self.Extent`))))
  (`KismetSystemLibrary.DrawDebugSphere` _location 4.0 12 (`KismetMathLibrary.SelectColor` (struct :`R` 0.04279 :`G` 0.286458 :`A` 1.0) (struct :`R` 0.229167 :`B` 0.00192 :`A` 1.0) (`ActorComponent.ComponentHasTag` _hitcomponent "Paintable")) 0.01 4.0)
  (bind _asstatic_mesh_component (cast `StaticMeshComponent` _hitcomponent))
  (bind (_min _max) (`StaticMeshComponent.GetLocalBounds` _asstatic_mesh_component))
  (set `self.Extent` (* (/ (- _max _min) 2.0) (`SceneComponent.K2_GetComponentScale` _asstatic_mesh_component)))
  (return (`KismetMathLibrary.MakeVector2D` (`KismetMathLibrary.MapRangeClamped` (.x (`KismetMathLibrary.GreaterGreater_VectorRotator` (- _location (`KismetSystemLibrary.GetComponentBounds` _hitcomponent)) (`KismetMathLibrary.NegateRotator` (`SceneComponent.K2_GetComponentRotation` _hitcomponent)))) _returnvalue_x _extent_x 0.0 1.0) (`KismetMathLibrary.MapRangeClamped` (.y (`KismetMathLibrary.GreaterGreater_VectorRotator` (- _location (`KismetSystemLibrary.GetComponentBounds` _hitcomponent)) (`KismetMathLibrary.NegateRotator` (`SceneComponent.K2_GetComponentRotation` _hitcomponent)))) _returnvalue_y _extent_y 0.0 1.0)) true))

(fn `UserConstructionScript`
  (`parent.UserConstructionScript`))